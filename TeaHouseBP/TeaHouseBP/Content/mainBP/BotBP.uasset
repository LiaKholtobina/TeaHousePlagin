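; Enemy bot that wanders to random reachable points nearby and chases the main character once PawnSensing spots it.
; Tick drives the behavior through latent Delays, using AIMoveTo for both wandering and pursuit.
; Reaching the character plays the bot animation and clears the sighting flag.
; While chasing, a box overlap flag gates delayed Demag calls on the character, independent of the move finishing.
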(event OnSeePawn(PawnSensing)
  (params (Pawn :type Pawn%20Object%20Reference))
  (bind _asmain_character (Utilities|Casting|CastTomainCharacter Pawn))
  (Variables|Default|Setsee%20pawn true)
  (Variables|Default|SetAs%20Main%20Character _asmain_character))

(event OnComponentBeginOverlap(Box)
  (params (OverlappedComponent :type Primitive%20Component%20Object%20Reference) (OtherActor :type Actor%20Object%20Reference) (OtherComp :type Primitive%20Component%20Object%20Reference) (OtherBodyIndex :type Integer) (bFromSweep :type Boolean) (SweepResult :type Hit%20Result%20Structure%20%28by%20ref%29))
  (Utilities|Casting|CastTomainCharacter OtherActor)
  (Variables|Default|Settouch%20pawn true))

(event OnComponentEndOverlap(Box)
  (params (OverlappedComponent :type Primitive%20Component%20Object%20Reference) (OtherActor :type Actor%20Object%20Reference) (OtherComp :type Primitive%20Component%20Object%20Reference) (OtherBodyIndex :type Integer))
  (Utilities|Casting|CastTomainCharacter OtherActor)
  (Variables|Default|Settouch%20pawn false))

(event EventTick
  (params (DeltaSeconds :type Float%20%28single-precision%29))
  (Utilities|FlowControl|Delay 0.2)
  (if (Variables|Default|Getsee%20pawn)
    (Utilities|FlowControl|Sequence
      (:then_0
        (Utilities|FlowControl|Delay 1.0)
        (AI|AIMoveTo self "0, 0, 0" (Variables|Default|GetAs%20Main%20Character) 1e+01 false
          (:then
            (Components|Animation|PlayAnimation (Variables|Character|GetMesh) "/Game/Models/BotAnim_Anim.BotAnim_Anim" false)
            (Utilities|FlowControl|Sequence
              (:then_0
                (Variables|Default|Setsee%20pawn false))))))
      (:then_1
        (Utilities|FlowControl|Delay 0.2)
        (if (Variables|Default|Gettouch%20pawn)
          (Default|Demag (Variables|Default|GetAs%20Main%20Character)))))
    (else
      (Utilities|FlowControl|Delay 1.0)
      (AI|AIMoveTo self (.RandomLocation (AI|Navigation|GetRandomReachablePointinRadius (Transformation|GetActorLocation) 1e+03 0 0)) 0 5.0 false))))

(fn ConstructionScript)