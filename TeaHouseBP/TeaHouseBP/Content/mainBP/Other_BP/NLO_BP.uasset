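; NLO (UFO) actor that flies its static mesh along a spline while spinning it, starting on BeginPlay.
; One timeline drives spline time, setting the mesh's relative transform from the location and direction at that point.
; A second timeline, started in the same sequence, sets relative yaw with zero pitch and roll, so both timelines write the mesh's rotation.
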(event EventBeginPlay
  (bind _spline (Variables|Default|GetSpline))
  (Utilities|FlowControl|Sequence
    (:then_0
      (bind _newtrack_0 (Timeline|Timeline Play)
        (:Update
          (Transformation|SetRelativeTransform (Variables|Default|GetStaticMesh) (Math|Transform|MakeTransform (Spline|GetLocationatTime _spline _newtrack_0 "Local" false) (Math|Rotator|MakeRotator (.roll (Math|Conversions|RotationFromXVector (Class|SplineComponent|GetDirectionatTime _spline _newtrack_0 "Local" false))) (.pitch (Math|Conversions|RotationFromXVector (Class|SplineComponent|GetDirectionatTime _spline _newtrack_0 "Local" false))) (.yaw (Math|Conversions|RotationFromXVector (Class|SplineComponent|GetDirectionatTime _spline _newtrack_0 "Local" false)))) "1.000000,1.000000,1.000000") false false))))
    (:then_1
      (bind _newtrack_0_2 (Timeline|Timeline_0 Play)
        (:Update
          (Transformation|SetRelativeRotation (Variables|Default|GetStaticMesh) (Math|Rotator|MakeRotator 0.0 0.0 _newtrack_0_2) false false))))))

(fn ConstructionScript)