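; A laser barrier actor that calls Demag on the main character when it crosses either of two beams.
; Every Tick, a shared LineTraceF function runs from each of two Arrow components, tracing a short, fixed distance along the arrow's forward vector against Pawn objects.
; A hit that casts to mainCharacter triggers Demag on each frame of contact, with no cooldown in this Blueprint.
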(event EventTick
  (params (DeltaSeconds :type Float%20%28single-precision%29))
  (Utilities|FlowControl|Sequence
    (:then_0
      (CallFunction|LineTraceF (Variables|Default|GetArrow)))
    (:then_1
      (CallFunction|LineTraceF (Variables|Default|GetArrow1)))))

(fn ConstructionScript)

(fn LineTraceF
  (params (Target :type Scene%20Component%20Object%20Reference))
  (bind _returnvalue (Transformation|GetWorldLocation Target))
  (bind _outhit (Collision|LineTraceForObjects _returnvalue (+ _returnvalue (* (Math|Vector|GetForwardVector Target) 4e+02)) (Utilities|Array|MakeArray "ObjectTypeQuery3") false 0 "None"))
  (bind _asmain_character (Utilities|Casting|CastTomainCharacter (.hitactor _outhit)))
  (Default|Demag _asmain_character))