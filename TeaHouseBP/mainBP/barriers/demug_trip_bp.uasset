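; Damage trap barrier that repeatedly calls Demag on the main character while it stands inside the Box trigger.
; Overlap lights the Cube orange through ChangeMatComponent and starts a looping one-second timer.
; Each tick briefly flashes the returned material red and triggers Demag at the same moment.
; Leaving the Box zeroes the glow intensity and clears the timer; the Destrroy event is an empty stub.
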(event OnComponentBeginOverlap(Box)
  (params (OverlappedComponent :type Primitive%20Component%20Object%20Reference) (OtherActor :type Actor%20Object%20Reference) (OtherComp :type Primitive%20Component%20Object%20Reference) (OtherBodyIndex :type Integer) (bFromSweep :type Boolean) (SweepResult :type Hit%20Result%20Structure%20%28by%20ref%29))
  ;[1 1 1] Изменение цвета
  (bind _asmain_character (Utilities|Casting|CastTomainCharacter OtherActor))
  (bind _returnvalue (Default|ChangeMatF (Variables|Default|GetChangeMatComponent) (Variables|Default|GetCube) 5e+01 "(R=1.000000,G=0.203922,B=0.000000,A=1.000000)"))
  ;[1 1 1] таймер
  (bind _returnvalue_2 (Utilities|Time|SetTimerbyEvent (delegate Custom|Demag_func) 1.0 true)))

(event OnComponentEndOverlap(Box)
  (params (OverlappedComponent :type Primitive%20Component%20Object%20Reference) (OtherActor :type Actor%20Object%20Reference) (OtherComp :type Primitive%20Component%20Object%20Reference) (OtherBodyIndex :type Integer))
  ;[1 1 1] Изменение цвета
  (Utilities|Casting|CastTomainCharacter OtherActor)
  (Default|ChangeMatF (Variables|Default|GetChangeMatComponent) (Variables|Default|GetCube) 0.0 "(R=0.989583,G=1.000000,B=1.000000,A=1.000000)")
  ;[1 1 1] таймер
  (Utilities|Time|ClearandInvalidateTimerbyHandle (stale OnComponentBeginOverlap(Box) _returnvalue_2)))

(event Custom|Demag_func
  ;[1 1 1] таймер
  (Utilities|FlowControl|Sequence
    (:then_0
      (Rendering|Material|SetVectorParameterValue (stale OnComponentBeginOverlap(Box) _returnvalue) "Color" "(R=1.000000,G=0.000000,B=0.000000,A=1.000000)" :!class /Script/Engine.MaterialInstanceDynamic)
      (Utilities|FlowControl|Delay 0.2)
      (Rendering|Material|SetVectorParameterValue (stale OnComponentBeginOverlap(Box) _returnvalue) "Color" "(R=1.000000,G=0.203994,B=0.000000,A=1.000000)" :!class /Script/Engine.MaterialInstanceDynamic))
    (:then_1
      (Default|Demag (stale OnComponentBeginOverlap(Box) _asmain_character)))))

(event EventDestrroy
  ;[1 1 1] Изменение цвета
)

(event EventBeginPlay
  (Default|ChangeMatF (Variables|Default|GetChangeMatComponent) (Variables|Default|GetCube) 0.0 "(R=0.000000,G=0.000000,B=0.000000,A=1.000000)"))

(fn ConstructionScript)